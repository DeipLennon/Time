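; BP_AssetPreview is the placement preview for the build system, showing whether an asset can be placed at its current spot.
; The construction script applies the Mesh variable to its StaticMesh component.
; Every tick it polls that component for overlapping components, setting CanPlaced to false with a red material when any exist, otherwise true with a green one.
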(event `self.ReceiveTick`
  (params (DeltaSeconds :type "Float (single-precision)"))
  (bind _staticmesh (`self.StaticMesh`))
  (if (> (`KismetArrayLibrary.Array_Length` (`PrimitiveComponent.GetOverlappingComponents` (`self.StaticMesh`))) 0)
    (`PrimitiveComponent.SetMaterial` _staticmesh 0 "/Game/Materials/M_Red.M_Red")
    (set `self.CanPlaced` false)
    (else
      (`PrimitiveComponent.SetMaterial` _staticmesh 0 "/Game/Materials/M_Green.M_Green")
      (set `self.CanPlaced` true))))

(fn `UserConstructionScript`
  (`StaticMeshComponent.SetStaticMesh` (`self.StaticMesh`) (`self.Mesh`)))