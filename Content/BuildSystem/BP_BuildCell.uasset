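; BP_BuildCell is a build-system cell that switches between a floor look and a default grid look.
; SetAsFloor sets the IsFloor flag and applies the passed material to the first slot of its StaticMesh, skipping the change if that material is already shown on a floor cell.
; SetAsDefault clears the flag and restores M_Grid, acting only when the cell is currently a floor.
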(fn `SetAsDefault`
  (if (`self.IsFloor`)
    (set `self.IsFloor` false)
    (`PrimitiveComponent.SetMaterial` (`self.StaticMesh`) 0 "/Game/Materials/M_Grid.M_Grid")))

(fn `SetAsFloor`
  (params (Material :type "MaterialInterface Object Reference"))
  (if (or (not (`self.IsFloor`)) (!= Material (`PrimitiveComponent.GetMaterial` (`self.StaticMesh`) 0)))
    (set `self.IsFloor` true)
    (`PrimitiveComponent.SetMaterial` (`self.StaticMesh`) 0 Material)))

(fn `UserConstructionScript`)