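; BP_FloorPreviw is a floor preview for the build system, showing a green or red mesh.
; On BeginPlay it finds the BP_GridManager, caches it and scales its static mesh to the grid's CellScale.
; The construction script picks M_Green or M_Red from the IsDraw flag, so the color is set at construction rather than updated in the event graph.
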(event `self.ReceiveBeginPlay`
  (bind _returnvalue (`GameplayStatics.GetActorOfClass` "/Game/BuildSystem/BP_GridManager.BP_GridManager_C"))
  (bind _output_get (set `self.GridManagerRef` _returnvalue))
  (`SceneComponent.SetWorldScale3D` (`self.StaticMesh`) (`/Game/BuildSystem/BP_GridManager.CellScale` _output_get)))

(fn `UserConstructionScript`
  (bind _staticmesh (`self.StaticMesh`))
  (if (`self.IsDraw`)
    (`PrimitiveComponent.SetMaterial` _staticmesh 0 "/Game/Materials/M_Green.M_Green")
    (else
      (`PrimitiveComponent.SetMaterial` _staticmesh 0 "/Game/Materials/M_Red.M_Red"))))