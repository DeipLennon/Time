(fn `GetBlockByCoordinate`
  (params (Coordinate :type "Vector2D Structure"))
  (returns (Output :type "/Game/BuildSystem/BP_BuildCell Object Reference"))
  (bind (_x _y) (`KismetMathLibrary.BreakVector2D` Coordinate))
  (return (`|GetArrayItem` (`.X_6_F1ED44F74C9CDECC8B553989EB08641F` (break `/Game/BuildSystem/S_Coordinate` (`|GetArrayItem` (`self.CoordinateGrid`) (`KismetMathLibrary.FTrunc` _y)))) (`KismetMathLibrary.FTrunc` _x))))

(fn `GetBlockLocation`
  (params (Location :type "Vector Structure"))
  (returns (OutLocation :type "Vector Structure"))
  (locals (Possition :type "Vector Structure") (Distance :type "Float (double-precision)"))
  (bind _returnvalue (`self.K2_GetActorLocation` (`|GetArrayItem` (`self.Cells`))))
  (set `local.Possition` _returnvalue)
  (set `local.Distance` (`KismetMathLibrary.Vector_Distance` Location _returnvalue))
  (for _array_element (`self.Cells`)
    (bind _returnvalue_2 (`self.K2_GetActorLocation` _array_element))
    (bind _returnvalue_3 (`KismetMathLibrary.Vector_Distance` _returnvalue_2 Location))
    (if (< _returnvalue_3 (`local.Distance`))
      (set `local.Possition` _returnvalue_2)
      (set `local.Distance` _returnvalue_3)))
  (return (`local.Possition`)))

(fn `MakeGrid`
  (locals (Offset :type "Float (double-precision)") (InArray :type "Array of /Game/BuildSystem/BP_BuildCell Object Reference"))
  (bind _cells (`self.Cells`))
  (bind _cellsize (`self.CellSize`))
  (bind _cellsize_2 (`self.CellSize`))
  (bind _returnvalue (`KismetMathLibrary.FTrunc` (`local.Offset`)))
  (bind _returnvalue_2 (- (`self.GridSize`) 1))
  (bind _returnvalue_3 (/ (`KismetMathLibrary.Conv_IntToDouble` (`self.CellSize`)) 100.0))
  (bind _returnvalue_4 (`KismetMathLibrary.MakeVector` _returnvalue_3 _returnvalue_3 1.0))
  (for _ _cells
    (`self.K2_DestroyActor`))
  (`KismetArrayLibrary.Array_Clear` _cells)
  (set `local.Offset` (- (* (* (`self.GridSize`) _cellsize) 0.5) (* _cellsize 0.5)))
  (`KismetArrayLibrary.Array_Clear` (`self.CoordinateGrid`))
  (for _index (range (+ _returnvalue_2 1))
    (`KismetArrayLibrary.Array_Clear` (`local.InArray`))
    (for _index_2 (range (+ _returnvalue_2 1))
      (set `self.CellScale` _returnvalue_4)
      (bind _returnvalue_5 (`|SpawnActorFromClass` "/Game/BuildSystem/BP_BuildCell.BP_BuildCell_C" (`KismetMathLibrary.MakeTransform` (`KismetMathLibrary.MakeVector` (`KismetMathLibrary.Conv_IntToDouble` (- (* _index_2 _cellsize_2) _returnvalue)) (`KismetMathLibrary.Conv_IntToDouble` (- (* _cellsize_2 _index) _returnvalue)) 0.1) (struct) _returnvalue_4) "AlwaysSpawn" "OverrideRootScale" null (`KismetMathLibrary.MakeVector2D` (`KismetMathLibrary.Conv_IntToDouble` _index_2) (`KismetMathLibrary.Conv_IntToDouble` _index)) null))
      (`KismetArrayLibrary.Array_Add` (`self.Cells`) _returnvalue_5)
      (`KismetArrayLibrary.Array_Insert` (`local.InArray`) _returnvalue_5 _index_2))
    (`KismetArrayLibrary.Array_Insert` (`self.CoordinateGrid`) (make `/Game/BuildSystem/S_Coordinate` (`local.InArray`)) _index)))

(fn `UserConstructionScript`)