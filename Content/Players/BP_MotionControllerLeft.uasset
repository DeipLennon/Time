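; BP_MotionControllerLeft is the left motion controller, serving as the mount for the grid and paint settings panels.
; Each spawn function destroys the other panel, then toggles its own by destroying it or spawning and attaching it to WidgetSocet.
; ApplyGridSettings closes the grid panel, passes the grid and cell sizes to BP_GridManager, and calls MakeGrid.
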(fn `ApplyGridSettings`
  (params (GridSize :type Integer) (CellSize :type Integer))
  (`self.K2_DestroyActor` (`self.GridSettingWidgetRef`))
  (set `self.GridSettingWidgetRef` null)
  (bind _returnvalue (`GameplayStatics.GetActorOfClass` "/Game/BuildSystem/BP_GridManager.BP_GridManager_C"))
  (set `/Game/BuildSystem/BP_GridManager.GridSize` GridSize _returnvalue)
  (set `/Game/BuildSystem/BP_GridManager.CellSize` CellSize _returnvalue)
  (`/Game/BuildSystem/BP_GridManager.MakeGrid` _returnvalue))

(fn `SpawnGridSettings`
  (bind _paintsettingwidgetref (`self.PaintSettingWidgetRef`)
    (:`then`
      (`self.K2_DestroyActor` _paintsettingwidgetref))
    (:`else`
      _))
  (bind _gridsettingwidgetref (`self.GridSettingWidgetRef`)
    (:`then`
      (`self.K2_DestroyActor` _gridsettingwidgetref))
    (:`else`
      (bind _returnvalue (`|SpawnActorFromClass` "/Game/Widgets/BP_GridSettings.BP_GridSettings_C" (`KismetMathLibrary.MakeTransform` (0.0 0.0 0.0) (struct :`Yaw` 180.0) (0.4 0.4 0.4)) "Undefined" "OverrideRootScale" null null))
      (bind _output_get (set `self.GridSettingWidgetRef` _returnvalue))
      (`self.K2_AttachToComponent` _output_get (`self.WidgetSocet`) "None" "KeepRelative" "KeepRelative" "KeepWorld" true))))

(fn `SpawnPaintSettings`
  (bind _gridsettingwidgetref (`self.GridSettingWidgetRef`)
    (:`then`
      (`self.K2_DestroyActor` _gridsettingwidgetref))
    (:`else`
      _))
  (bind _paintsettingwidgetref (`self.PaintSettingWidgetRef`)
    (:`then`
      (`self.K2_DestroyActor` _paintsettingwidgetref))
    (:`else`
      (bind _returnvalue (`|SpawnActorFromClass` "/Game/Widgets/BP_PaintSettings.BP_PaintSettings_C" (`KismetMathLibrary.MakeTransform` (30.0 0.0 0.0) (struct :`Yaw` 180.0) (0.4 0.4 0.4)) "Undefined" "OverrideRootScale" null null))
      (bind _output_get (set `self.PaintSettingWidgetRef` _returnvalue))
      (`self.K2_AttachToComponent` _output_get (`self.WidgetSocet`) "None" "KeepRelative" "KeepRelative" "KeepWorld" true))))

(fn `UserConstructionScript`)