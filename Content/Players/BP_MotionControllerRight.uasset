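; Right-hand VR motion controller that serves as the building tool on a BP_GridManager grid and clicks widgets.
; A per-tick line trace finds the targeted cell, moves the asset preview or highlights placed assets through custom depth.
; The trigger drags out previewed rectangles to draw or delete floor, or places assets, which can also be grabbed as ghosts or removed.
; Wall functions rebuild BP_Wall actors along floor-cell edges by checking neighboring cells.
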(event `self.ReceiveBeginPlay`
  (set `self.As BP Pawn` (cast `/Game/Players/BP_VrPawn` (`self.GetOwner`) :!pure true))
  (bind _returnvalue (`GameplayStatics.GetActorOfClass` "/Game/Players/BP_MotionControllerLeft.BP_MotionControllerLeft_C"))
  (set `self.IgnoreActors` (`|MakeArray` _returnvalue (`self.As BP Pawn`) :!type "Actor Object Reference"))
  (bind _returnvalue_2 (`GameplayStatics.GetActorOfClass` "/Game/BuildSystem/BP_GridManager.BP_GridManager_C"))
  (set `self.GridManagerRef` _returnvalue_2))

(event `self.ReceiveTick`
  (params (DeltaSeconds :type "Float (single-precision)"))
  (bind _motioncontroller (`self.MotionController`))
  (bind _as_bp_build_asset (`self.As BP Build Asset`))
  (bind _as_bp_build_asset_2 (`self.As BP Build Asset`))
  (bind _returnvalue (`SceneComponent.K2_GetComponentLocation` _motioncontroller))
  (bind _outhit (`KismetSystemLibrary.LineTraceSingle` _returnvalue (+ _returnvalue (* (* (`SceneComponent.GetUpVector` _motioncontroller) -1.0) 1000.0)) "TraceTypeQuery1" false (`self.IgnoreActors`)))
  (bind (_bblockinghit _binitialoverlap _time _distance _location _impactpoint _normal _impactnormal _physmat _hitactor) (`GameplayStatics.BreakHitResult` _outhit))
  (bind _asbp_build_cell (cast `/Game/BuildSystem/BP_BuildCell` _hitactor)
    (:`then`
      (set `self.As BP Build Block` _asbp_build_cell)
      (set `self.IsPointerOnBlock` true)
      (`|ExecutionSequence`
        (:`then_0`
          (if (`self.IsFloorCreating`)
            (`self.BuildingFloor`)))
        (:`then_1`
          (if (`|EnumEquality` (`self.CurrentPaintTool`) "NewEnumerator5")
            (`/Engine/EditorBlueprintResources/StandardMacros.IsValid` _as_bp_build_asset_2
              (:`Is Valid`
                (`PrimitiveComponent.SetRenderCustomDepth` (`/Game/BuildSystem/BP_BuildAsset.StaticMesh` _as_bp_build_asset_2) false))
              (:`Is Not Valid`
                _))
            (`SceneComponent.SetVisibility` (`/Game/BuildSystem/BP_AssetPreview.StaticMesh` (`self.Preview`)) true false)
            (`self.K2_SetActorLocation` (`self.Preview`) (`/Game/BuildSystem/BP_GridManager.GetBlockLocation` (`self.GridManagerRef`) _location) false true)))))
    (:`CastFailed`
      (if (`|EnumEquality` (`self.CurrentPaintTool`) "NewEnumerator5")
        (set `self.IsPointerOnBlock` false)
        (`SceneComponent.SetVisibility` (`/Game/BuildSystem/BP_AssetPreview.StaticMesh` (`self.Preview`)) false false)
        (bind _asbp_build_asset (cast `/Game/BuildSystem/BP_BuildAsset` _hitactor)
          (:`then`
            (set `self.As BP Build Asset` _asbp_build_asset)
            (`PrimitiveComponent.SetRenderCustomDepth` (`/Game/BuildSystem/BP_BuildAsset.StaticMesh` _asbp_build_asset) true))
          (:`CastFailed`
            (`/Engine/EditorBlueprintResources/StandardMacros.IsValid` _as_bp_build_asset
              (:`Is Valid`
                (`PrimitiveComponent.SetRenderCustomDepth` (`/Game/BuildSystem/BP_BuildAsset.StaticMesh` _as_bp_build_asset) false)))))))))

(event `TriggerPress`
  (`WidgetInteractionComponent.PressPointerKey` (`self.WidgetInteraction`) "LeftMouseButton")
  (switch `/Game/BuildSystem/E_PaintTools` (`self.CurrentPaintTool`)
    (:`NewEnumerator3`
      (set `self.IsDraw` true)
      (`self.StartCreateFloor`))
    (:`NewEnumerator4`
      (set `self.IsDraw` false)
      (`self.StartCreateFloor`))
    (:`NewEnumerator5`
      (`self.CreateAsset` false))))

(event `RemoveAsset`
  (bind _as_bp_build_asset (`self.As BP Build Asset`))
  (if (`self.IsGrabing`)
    (set `self.IsGrabing` false)
    (`self.StopGrab`)
    (else
      (`/Engine/EditorBlueprintResources/StandardMacros.IsValid` _as_bp_build_asset
        (:`Is Valid`
          (`self.K2_DestroyActor` _as_bp_build_asset)
          (set `self.As BP Build Asset` null))))))

(event `AButtonPress`
  (`self.RemoveAsset`))

(event `TriggerRelease`
  (`WidgetInteractionComponent.ReleasePointerKey` (`self.WidgetInteraction`) "LeftMouseButton")
  (switch `/Game/BuildSystem/E_PaintTools` (`self.CurrentPaintTool`)
    (:`NewEnumerator3`
      (`self.StopCreateFloor`))
    (:`NewEnumerator4`
      (`self.StopCreateFloor`))))

(event `StartGrab`
  (bind _as_bp_build_asset (`self.As BP Build Asset`))
  (`/Engine/EditorBlueprintResources/StandardMacros.IsValid` _as_bp_build_asset
    (:`Is Valid`
      (set `self.IsGrabing` true)
      (bind _output_get (set `self.Transform` (`self.GetTransform` _as_bp_build_asset)))
      (`self.K2_DestroyActor` _as_bp_build_asset)
      (set `self.As BP Build Asset` null)
      (bind _returnvalue (`|SpawnActorFromClass` "/Game/BuildSystem/BP_Ghost.BP_Ghost_C" _output_get "Undefined" "OverrideRootScale" null (`self.AssetMesh`) null))
      (set `self.GhostRef` _returnvalue))))

(event `SpawnAsset`
  (bind _preview (`self.Preview`))
  (`/Engine/EditorBlueprintResources/StandardMacros.IsValid` _preview
    (:`Is Valid`
      (`KismetArrayLibrary.Array_RemoveItem` (`self.IgnoreActors`) _preview)
      (`self.K2_DestroyActor` _preview))
    (:`Is Not Valid`
      _))
  (bind _returnvalue (`|SpawnActorFromClass` "/Game/BuildSystem/BP_AssetPreview.BP_AssetPreview_C" (`KismetMathLibrary.MakeTransform` (0.0 0.0 0.0)) "Undefined" "OverrideRootScale" null (`self.AssetMesh`) null))
  (bind _output_get (set `self.Preview` _returnvalue))
  (`KismetArrayLibrary.Array_Add` (`self.IgnoreActors`) _output_get)
  (`KismetSystemLibrary.PrintString` "Hello"))

(event `StopGrab`
  (bind _ghostref (`self.GhostRef`))
  (if (`self.IsGrabing`)
    (bind _result (`self.CreateAsset` false))
    (if (not _result)
      (`self.CreateAsset` true (`self.Transform`) :!label _label))
    (else
      (goto _label)))
  (`/Engine/EditorBlueprintResources/StandardMacros.IsValid` _ghostref
    (:`Is Valid`
      (`self.K2_DestroyActor` _ghostref)
      (set `self.IsGrabing` false))))

(event `RotateLeft`
  (bind _preview (`self.Preview`))
  (`self.K2_SetActorRotation` _preview (`KismetMathLibrary.ComposeRotators` (`self.K2_GetActorRotation` _preview) (struct :`Yaw` -15.0)) false))

(event `RotateRight`
  (bind _preview (`self.Preview`))
  (`self.K2_SetActorRotation` _preview (`KismetMathLibrary.ComposeRotators` (`self.K2_GetActorRotation` _preview) (struct :`Yaw` 15.0)) false))

(fn `BuildingFloor`
  (bind _returnvalue (`self.GetTransform` (`self.As BP Build Block`)))
  (if (`self.IsPointerOnBlock`)
    (if (not (`self.IsFirstCell`))
      (if (not (== _returnvalue (`self.LastCellTransform`)))
        (for _array_element (`self.FloorCellsPreview`)
          (`self.K2_DestroyActor` _array_element))
        (`KismetArrayLibrary.Array_Clear` (`self.FloorCellsPreview`))
        (bind _output_get (set `self.LastCellTransform` _returnvalue))
        (bind _returnvalue_2 (`|SpawnActorFromClass` "/Game/BuildSystem/BP_FloorPreviw.BP_FloorPreviw_C" _output_get "Undefined" "OverrideRootScale" null (`self.IsDraw`) null))
        (`KismetArrayLibrary.Array_Add` (`self.FloorCellsPreview`) _returnvalue_2)
        (`self.ProectionFloor`)))))

(fn `CanselCreatingFloor`
  (bind _floorcellspreview (`self.FloorCellsPreview`))
  (set `self.IsFloorCreating` false)
  (set `self.IsFirstCell` true)
  (`KismetArrayLibrary.Array_Add` _floorcellspreview (`self.FirstFloorCell`))
  (for _array_element _floorcellspreview
    (`self.K2_DestroyActor` _array_element))
  (`KismetArrayLibrary.Array_Clear` _floorcellspreview))

(fn `CreateAsset`
  (params (UseTransform :type Boolean) (Transform :type "Transform Structure"))
  (returns (Result :type Boolean))
  (if UseTransform
    _
    (elif (`/Game/BuildSystem/BP_AssetPreview.CanPlaced` (`self.Preview`))
      _
      (else
        (return false))))
  (`|SpawnActorFromClass` "/Game/BuildSystem/BP_BuildAsset.BP_BuildAsset_C" (`KismetMathLibrary.SelectTransform` Transform (`self.GetTransform` (`self.Preview`)) UseTransform) "Undefined" "OverrideRootScale" null (`self.AssetMesh`) null)
  (return true))

(fn `MakeWall`
  (bind _gridmanagerref (`self.GridManagerRef`))
  (bind _wallscale (`self.WallScale`))
  (bind _wallmaterial (`self.WallMaterial`))
  (bind _returnvalue (`KismetMathLibrary.Conv_IntToDouble` (- (`/Game/BuildSystem/BP_GridManager.GridSize` (`self.GridManagerRef`)) 1)))
  (bind _returnvalue_2 (/ (`KismetMathLibrary.Conv_IntToDouble` (`/Game/BuildSystem/BP_GridManager.CellSize` (`self.GridManagerRef`))) 2.0))
  (bind _outactors (`GameplayStatics.GetAllActorsOfClass` "/Game/BuildSystem/BP_Wall.BP_Wall_C"))
  (if (> (`KismetArrayLibrary.Array_Length` _outactors) 0)
    (for _array_element _outactors
      (`self.K2_DestroyActor` _array_element)))
  (bind _outactors_2 (`GameplayStatics.GetAllActorsOfClass` "/Game/BuildSystem/BP_BuildCell.BP_BuildCell_C"))
  (for _array_element_2 _outactors_2
    (if (`/Game/BuildSystem/BP_BuildCell.IsFloor` _array_element_2)
      (bind (_x _y) (`KismetMathLibrary.BreakVector2D` (`/Game/BuildSystem/BP_BuildCell.Coordinate` _array_element_2)))
      (bind _returnvalue_3 (+ _x 1.0))
      (if (<= _returnvalue_3 _returnvalue)
        (bind _output (`/Game/BuildSystem/BP_GridManager.GetBlockByCoordinate` _gridmanagerref (`KismetMathLibrary.MakeVector2D` _returnvalue_3 _y)))
        (if (not (`/Game/BuildSystem/BP_BuildCell.IsFloor` _output))
          (`|SpawnActorFromClass` "/Game/BuildSystem/BP_Wall.BP_Wall_C" (`KismetMathLibrary.MakeTransform` (- (`self.K2_GetActorLocation` _output) (`KismetMathLibrary.MakeVector` _returnvalue_2)) (struct :`Yaw` 90.0) _wallscale) "Undefined" "OverrideRootScale" null _wallmaterial null))
        (bind _returnvalue_4 (- _x 1.0))
        (bind _output_2 (`/Game/BuildSystem/BP_GridManager.GetBlockByCoordinate` _gridmanagerref (`KismetMathLibrary.MakeVector2D` _returnvalue_4 _y) :!label _label))
        (if (not (`/Game/BuildSystem/BP_BuildCell.IsFloor` _output_2))
          (`|SpawnActorFromClass` "/Game/BuildSystem/BP_Wall.BP_Wall_C" (`KismetMathLibrary.MakeTransform` (+ (`self.K2_GetActorLocation` _output_2) (`KismetMathLibrary.MakeVector` _returnvalue_2)) (struct :`Yaw` -90.0) _wallscale) "Undefined" "OverrideRootScale" null _wallmaterial null))
        (bind _returnvalue_5 (+ _y 1.0))
        (bind _output_3 (`/Game/BuildSystem/BP_GridManager.GetBlockByCoordinate` _gridmanagerref (`KismetMathLibrary.MakeVector2D` _x _returnvalue_5) :!label _label_2))
        (if (not (`/Game/BuildSystem/BP_BuildCell.IsFloor` _output_3))
          (`|SpawnActorFromClass` "/Game/BuildSystem/BP_Wall.BP_Wall_C" (`KismetMathLibrary.MakeTransform` (- (`self.K2_GetActorLocation` _output_3) (`KismetMathLibrary.MakeVector` 0.0 _returnvalue_2)) (struct :`Yaw` 180.0) _wallscale) "Undefined" "OverrideRootScale" null _wallmaterial null))
        (bind _returnvalue_6 (- _y 1.0))
        (bind _output_4 (`/Game/BuildSystem/BP_GridManager.GetBlockByCoordinate` _gridmanagerref (`KismetMathLibrary.MakeVector2D` _x _returnvalue_6) :!label _label_3))
        (if (not (`/Game/BuildSystem/BP_BuildCell.IsFloor` _output_4))
          (`|SpawnActorFromClass` "/Game/BuildSystem/BP_Wall.BP_Wall_C" (`KismetMathLibrary.MakeTransform` (+ (`self.K2_GetActorLocation` _output_4) (`KismetMathLibrary.MakeVector` 0.0 _returnvalue_2)) (struct) _wallscale) "Undefined" "OverrideRootScale" null _wallmaterial null))
        (elif (>= _returnvalue_4 0.0)
          (goto _label)
          (elif (<= _returnvalue_5 _returnvalue)
            (goto _label_2)
            (elif (>= _returnvalue_6 0.0)
              (goto _label_3))))))))

(fn `ProectionFloor`
  (bind (_x _y) (`KismetMathLibrary.BreakVector2D` (`/Game/BuildSystem/BP_BuildCell.Coordinate` (`self.As BP Build Block`))))
  (bind _x_2 (.x (.location (`self.LastCellTransform`))))
  (bind _y_2 (.y (.location (`self.LastCellTransform`))))
  (bind _x_3 (.x (.location (`self.FirstCellTransform`))))
  (bind _y_3 (.y (.location (`self.FirstCellTransform`))))
  (bind _returnvalue (`KismetMathLibrary.FTrunc` _y))
  (bind _returnvalue_2 (`KismetMathLibrary.FTrunc` _x))
  (`|ExecutionSequence`
    (:`then_0`
      (if (== _x_3 _x_2)
        (set `self.XDirection` "NewEnumerator0")
        (elif (< _x_3 _x_2)
          (set `self.XDirection` "NewEnumerator1")
          (else
            (set `self.XDirection` "NewEnumerator2")))))
    (:`then_1`
      (if (== _y_3 _y_2)
        (set `self.YDirection` "NewEnumerator0")
        (elif (< _y_3 _y_2)
          (set `self.YDirection` "NewEnumerator1")
          (else
            (set `self.YDirection` "NewEnumerator2")))))
    (:`then_2`
      (set `self.XSize` (`KismetMathLibrary.FTrunc` (/ (`KismetMathLibrary.Abs` (- _x_3 _x_2)) (`/Game/BuildSystem/BP_GridManager.CellSize` (`self.GridManagerRef`)))))
      (set `self.YSize` (`KismetMathLibrary.FTrunc` (/ (`KismetMathLibrary.Abs` (- _y_3 _y_2)) (`/Game/BuildSystem/BP_GridManager.CellSize` (`self.GridManagerRef`)))))
      (`KismetArrayLibrary.Array_Clear` (`self.CellsToFloor`))
      (for _index (range (+ (`self.YSize`) 1))
        (for _index_2 (range (+ (`self.XSize`) 1))
          (bind _output (`/Game/BuildSystem/BP_GridManager.GetBlockByCoordinate` (`self.GridManagerRef`) (`KismetMathLibrary.MakeVector2D` (`KismetMathLibrary.Conv_IntToDouble` (`KismetMathLibrary.SelectInt` (+ _index_2 _returnvalue_2) (- _returnvalue_2 _index_2) (`|EnumEquality` (`self.XDirection`) "NewEnumerator2"))) (`KismetMathLibrary.Conv_IntToDouble` (`KismetMathLibrary.SelectInt` (+ _index _returnvalue) (- _returnvalue _index) (`|EnumEquality` (`self.YDirection`) "NewEnumerator2"))))))
          (`KismetArrayLibrary.Array_Add` (`self.CellsToFloor`) _output)
          (bind _returnvalue_3 (`|SpawnActorFromClass` "/Game/BuildSystem/BP_FloorPreviw.BP_FloorPreviw_C" (`self.GetTransform` _output) "Undefined" "OverrideRootScale" null (`self.IsDraw`) null))
          (`KismetArrayLibrary.Array_Add` (`self.FloorCellsPreview`) _returnvalue_3))))))

(fn `RemoveWalls`
  (bind _outactors (`GameplayStatics.GetAllActorsOfClass` "/Game/BuildSystem/BP_Wall.BP_Wall_C"))
  (if (> (`KismetArrayLibrary.Array_Length` _outactors) 0)
    (for _array_element _outactors
      (`self.K2_DestroyActor` _array_element))))

(fn `SetWallScale`
  (params (Y :type "Float (double-precision)"))
  (bind _output_get (set `self.WallScale` (`KismetMathLibrary.MakeVector` (.x (`/Game/BuildSystem/BP_GridManager.CellScale` (`self.GridManagerRef`))) Y (.z (`/Game/BuildSystem/BP_GridManager.CellScale` (`self.GridManagerRef`))))))
  (`KismetSystemLibrary.PrintString` (`KismetStringLibrary.Conv_VectorToString` _output_get))
  (`self.MakeWall`))

(fn `StartCreateFloor`
  (if (`self.IsPointerOnBlock`)
    (if (`self.IsFirstCell`)
      (bind _output_get (set `self.FirstCellTransform` (`self.GetTransform` (`self.As BP Build Block`))))
      (set `self.IsFirstCell` false)
      (set `self.IsFloorCreating` true)
      (bind _returnvalue (`|SpawnActorFromClass` "/Game/BuildSystem/BP_FloorPreviw.BP_FloorPreviw_C" _output_get "Undefined" "OverrideRootScale" null (`self.IsDraw`) null))
      (set `self.FirstFloorCell` _returnvalue))))

(fn `StopCreateFloor`
  (bind _floorcellspreview (`self.FloorCellsPreview`))
  (set `self.IsFloorCreating` false)
  (set `self.IsFirstCell` true)
  (`KismetArrayLibrary.Array_Add` _floorcellspreview (`self.FirstFloorCell`))
  (for _array_element _floorcellspreview
    (`/Engine/EditorBlueprintResources/StandardMacros.IsValid` _array_element
      (:`Is Valid`
        (`self.K2_DestroyActor` _array_element))))
  (`KismetArrayLibrary.Array_Clear` _floorcellspreview)
  (for _array_element_2 (`self.CellsToFloor`)
    (if (`self.IsDraw`)
      (`/Game/BuildSystem/BP_BuildCell.SetAsFloor` _array_element_2 (`self.FloorMaterial`))
      (else
        (`/Game/BuildSystem/BP_BuildCell.SetAsDefault` _array_element_2)))))

(fn `UserConstructionScript`)